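; AI controller for the boss that starts the BT_Boss behavior tree on BeginPlay.
; PawnSensing sets the "seeingTarget?" blackboard flag when it sees any pawn, and nothing here clears it.
; An AI Perception sight handler for TargetActor and LastKnownLocation exists but is disconnected from the perception event.
; That handler also compares the sense class to AISenseConfig_Sight, a config class rather than a sense class.
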(event OnSeePawn(PawnSensing)
  (params (Pawn :type Pawn%20Object%20Reference))
  ;[0.15 0.15 0.15 0.5] 플레이어 센싱
  (AI|Components|Blackboard|SetValueasBool (AI|GetBlackboard 0) (Utilities|Name|MakeLiteralName "seeingTarget?") true))

(event OnTargetPerceptionUpdated(AIPerception)
  (params (Actor :type Actor%20Object%20Reference) (Stimulus :type AI%20Stimulus%20Structure))
  ;[0.15 0.15 0.15 0.5] AI Perception
)

(event EventBeginPlay
  ;[0.15 0.15 0.15 0.5] 행동트리 실행
  (AI|RunBehaviorTree "/Game/LSJ/Boss/BT_Boss.BT_Boss"))

(fn ConstructionScript)

(fn HandleSightSense
  (params (Actor :type Actor%20Object%20Reference) (Stimulus :type AI%20Stimulus%20Structure))
  (bind _returnvalue (Class|AIPerceptionSystem|GetSenseClassforStimulus Stimulus))
  (if (== _returnvalue "/Script/AIModule.AISenseConfig_Sight")
    (if (== Actor (Game|GetPlayerCharacter 0))
      (AI|Components|Blackboard|SetValueasObject (Variables|Default|GetBlackboard) (Utilities|Name|MakeLiteralName "TargetActor") (Utilities|SelectObject (Game|GetPlayerCharacter 0) 0 (.bsuccessfullysensed Stimulus)))
      (if (not (.bsuccessfullysensed Stimulus))
        (AI|Components|Blackboard|SetValueasVector (Variables|Default|GetBlackboard) (Utilities|Name|MakeLiteralName "LastKnownLocation") (.stimuluslocation Stimulus)))
      (else
        (return)))
    (else
      (return))))