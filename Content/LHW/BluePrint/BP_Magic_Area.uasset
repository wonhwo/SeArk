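; BP_Magic_Area is an actor that follows the mouse cursor near the player, apparently as a spell targeting area.
; BeginPlay picks one of two maximum ranges from the player character's OnChageKey, then snaps to the cursor's hit point at roughly foot height.
; Each Tick repeats that snap while the actor's current location is within range, otherwise placing it at maximum range toward the cursor.
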(event EventBeginPlay
  (bind _returnvalue (Game|GetPlayerController 0))
  (bind _hitresult (Game|Player|GetHitResultUnderCursorbyChannel _returnvalue "TraceTypeQuery1" true))
  (bind _impactpoint (Collision|BreakHitResult _hitresult))
  (bind (_x _y) (Math|Vector|BreakVector _impactpoint))
  (bind _asmyplayer_character (Utilities|Casting|CastToMyplayerCharacter (Game|GetPlayerCharacter 0)))
  (switch int (Variables|/Game/LHW/BluePrint/MyplayerCharacter.MyplayerCharacter_C|GetonChageKey _asmyplayer_character)
    (:1
      (Variables|Default|SetCDistance 4.5e+02))
    (:2
      (Variables|Default|SetCDistance 6e+02)))
  (Transformation|SetActorLocation (Math|Vector|MakeVector _x _y (- (.Z (Math|Vector|BreakVector (Transformation|GetActorLocation (Game|GetPlayerCharacter 0)))) 9e+01)) true false))

(event Collision|EventActorBeginOverlap
  (params (OtherActor :type Actor%20Object%20Reference)))

(event EventTick
  (params (DeltaSeconds :type Float%20%28single-precision%29))
  (bind _returnvalue (Game|GetPlayerController 0))
  (bind _returnvalue_2 (Game|GetPlayerCharacter 0))
  (bind _returnvalue_3 (Game|GetPlayerCharacter 0))
  (bind _cdistance (Variables|Default|GetCDistance))
  (bind _returnvalue_4 (Transformation|GetActorLocation _returnvalue_3))
  (bind _returnvalue_5 (Transformation|GetActorLocation _returnvalue_2))
  (bind _hitresult (Game|Player|GetHitResultUnderCursorbyChannel _returnvalue "TraceTypeQuery1" true))
  (bind _impactpoint (Collision|BreakHitResult _hitresult))
  (bind _z (Math|Vector|BreakVector _returnvalue_4))
  (bind (_x _y) (Math|Vector|BreakVector _impactpoint))
  (bind _returnvalue_6 (- _z 9e+01))
  (bind _returnvalue_7 (Math|Vector|MakeVector _x _y _returnvalue_6))
  (bind _returnvalue_8 (- _returnvalue_7 _returnvalue_5))
  (bind _returnvalue_9 (Math|Vector|Normalize _returnvalue_8))
  (bind _returnvalue_10 (* _returnvalue_9 _cdistance))
  (bind _returnvalue_11 (+ _returnvalue_5 _returnvalue_10))
  (if (<= (Math|Vector|Distance(Vector) (Transformation|GetActorLocation) _returnvalue_4) (Variables|Default|GetCDistance))
    (Transformation|SetActorLocation _returnvalue_7 true false)
    (else
      (Transformation|SetActorLocation (Math|Vector|MakeVector (.x _returnvalue_11) (.y _returnvalue_11) _returnvalue_6) true false)
      (Variables|Default|SetDistanceOve false))))

(fn ConstructionScript)