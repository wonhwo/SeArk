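; EnemySample is a boss-style test enemy that creates a boss health bar widget on BeginPlay.
; On overlap it rolls randomized damage for normal attack, meteor or ice colliders, each with its own base, and subtracts it straight from the widget's health value.
; Each hit spawns a BP_Damage actor carrying that damage, cycling through height offsets.
; Overlapping the player character applies massive damage to it.
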(event EventBeginPlay
  (bind _returnvalue (UserInterface|CreateWidget "/Game/LHW/ui/WBP_BossHealthBar.WBP_BossHealthBar_C"))
  (UserInterface|Viewport|AddtoViewport _returnvalue 0))

(event Collision|EventActorBeginOverlap
  (params (OtherActor :type Actor%20Object%20Reference))
  (bind _returnvalue (Transformation|GetActorTransform))
  (Utilities|FlowControl|Sequence
    (:then_0
      (Utilities|Casting|CastToBP_NormalAttack OtherActor)
      (Development|PrintString "평타")
      (Variables|Default|SetcurrentDamage (* (Math|Random|RandomFloatinRange 1.0 1.3999) 1e+03))
      (Variables|/Game/LHW/ui/WBP_BossHealthBar.WBP_BossHealthBar_C|SetBossCurrentHealth (stale EventBeginPlay _returnvalue) (- (Variables|/Game/LHW/ui/WBP_BossHealthBar.WBP_BossHealthBar_C|GetBossCurrentHealth (stale EventBeginPlay _returnvalue)) (Variables|Default|GetcurrentDamage)) :!label _label)
      (bind _returnvalue_2 (Game|SpawnActorfromClass "/Game/LHW/BluePrint/BP_Damage.BP_Damage_C" (Math|Transform|MakeTransform (Math|Vector|MakeVector (.x (.location _returnvalue)) (.y (.location _returnvalue)) (+ (.z (.location _returnvalue)) (Utilities|Array|Get(acopy) (Variables|Default|GetOffsets) (Variables|Default|Getindex)))) (.rotation _returnvalue) (.scale _returnvalue)) "Undefined" "MultiplyWithRoot" 0 (Variables|Default|GetcurrentDamage) 0))
      (Variables|Default|SetBp_damage _returnvalue_2)
      (if (== (Variables|Default|Getindex) 4)
        (Variables|Default|Setindex 0)
        (else
          (Variables|Default|Setindex (+ (Variables|Default|Getindex) 1)))))
    (:then_1
      (Utilities|Casting|CastToBP_MeteorCollider OtherActor)
      (Development|PrintString "메테오")
      (Variables|Default|SetcurrentDamage (* (Math|Random|RandomFloatinRange 1.0 1.3999) 1e+04))
      (goto _label))
    (:then_2
      (Utilities|Casting|CastToBP_IceCollider OtherActor)
      (Development|PrintString "얼음")
      (Variables|Default|SetcurrentDamage (* (Math|Random|RandomFloatinRange 1.0 1.3999) 5e+03))
      (goto _label))
    (:then_3
      (bind _asmyplayer_character (Utilities|Casting|CastToMyplayerCharacter OtherActor))
      (Game|Damage|ApplyDamage _asmyplayer_character 1e+05 0 self))))

(event EventTick
  (params (DeltaSeconds :type Float%20%28single-precision%29)))

(fn ConstructionScript)

(fn IfGetVector
  (bind _returnvalue (Transformation|GetActorRotation))
  (return (Math|Vector|GetUpVector _returnvalue) (Math|Vector|GetRightVector _returnvalue)))