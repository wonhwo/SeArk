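; Meteor skill actor that runs the player's cast, then drops a meteor at its own location.
; BeginPlay spawns a magic circle under the player and a cast-bar widget driven by a Timeline, which aborts through the character's SkillCanCel flag and calls its cooldown.
; On completion it spawns a ground circle and overhead portal, then the stone after a delay, while a second Timeline drives the HUD cooldown display.
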(event EventBeginPlay
  (bind _returnvalue (Game|GetPlayerCharacter 0))
  (bind _returnvalue_2 (Transformation|GetActorLocation))
  (bind (_x _y) (Math|Vector|BreakVector _returnvalue_2))
  (bind (_x_2 _y_2) (Math|Vector|BreakVector _returnvalue_2))
  (bind _returnvalue_3 (Transformation|GetActorLocation _returnvalue))
  (bind _returnvalue_4 (+ (.z _returnvalue_3) 5e+02))
  (bind _returnvalue_5 (+ (.z _returnvalue_3) 4.6e+02))
  (bind _returnvalue_6 (Math|Vector|MakeVector _x_2 _y_2 _returnvalue_4))
  (bind (_x_3 _y_3) (Math|Vector|BreakVector _returnvalue_6))
  (bind _returnvalue_7 (Math|Vector|MakeVector _x_3 _y_3 _returnvalue_5))
  (bind _asmyplayer_character (Utilities|Casting|CastToMyplayerCharacter (Game|GetPlayerCharacter 0)))
  (Variables|Default|SetOwnerCharacter _asmyplayer_character)
  (bind _returnvalue_8 (UserInterface|CreateWidget "/Game/LHW/ui/WBP_catingUi.WBP_catingUi_C"))
  (UserInterface|Viewport|AddtoViewport _returnvalue_8 0)
  (bind _returnvalue_9 (Game|SpawnActorfromClass "/Game/LHW/Magic_Circle_Creator/Blueprints/BP_MagicCircleCreatorADV.BP_MagicCircleCreatorADV_C" (Math|Transform|MakeTransform (Math|Vector|MakeVector (.x (Transformation|GetActorLocation _asmyplayer_character)) (.y (Transformation|GetActorLocation _asmyplayer_character)) (- (.z (Transformation|GetActorLocation _asmyplayer_character)) 85.0)) "0, 0, 0" "10.000000,10.000000,10.000000") "Undefined" "MultiplyWithRoot" 0 0))
  (bind _newtrack_0 (Timeline|Timeline Play)
    (:Update
      (if (Variables|/Game/LHW/BluePrint/MyplayerCharacter.MyplayerCharacter_C|GetSkillCanCel (Variables|Default|GetOwnerCharacter))
        (Animation|StopAnimMontage (Variables|Default|GetOwnerCharacter) (Animation|GetCurrentMontage (Variables|Default|GetOwnerCharacter) :!class /Script/Engine.Character))
        (Actor|DestroyActor _returnvalue_9)
        (Default|StartMovementPlayer (Variables|Default|GetOwnerCharacter))
        (Widget|RemovefromParent _returnvalue_8)
        (Default|CoolDownTeteor (Variables|Default|GetOwnerCharacter))
        (Timeline|Timeline Stop)
        (else
          (Utilities|IsValid _returnvalue_8
            (:Is%20Valid
              (Variables|/Game/LHW/ui/WBP_catingUi.WBP_catingUi_C|SetSkillCastTime _returnvalue_8 _newtrack_0))))))
    (:Finished
      (Actor|DestroyActor _returnvalue_9)
      (Widget|RemovefromParent _returnvalue_8)
      (bind _asmyplayer_character_2 (Utilities|Casting|CastToMyplayerCharacter (Game|GetPlayerCharacter 0)))
      (Utilities|FlowControl|Sequence
        (:then_0
          (Variables|/Game/LHW/BluePrint/MyplayerCharacter.MyplayerCharacter_C|SetisSkillCasting _asmyplayer_character_2 false)
          (bind _returnvalue_10 (Game|SpawnActorfromClass "/Game/LHW/Skill_Resouroes/Meteor/Meteor_circle.Meteor_circle_C" (Math|Transform|MakeTransform (Math|Vector|MakeVector _x _y (+ (.z _returnvalue_3) -8e+01)) "0, 0, 0" "2.000000,2.000000,2.000000") "Undefined" "MultiplyWithRoot" 0 0))
          (Variables|Default|SetgetMouseClick _returnvalue_7)
          (Game|SpawnActorfromClass "/Game/LHW/Skill_Resouroes/Meteor/Meteor_portal.Meteor_portal_C" (Math|Transform|MakeTransform _returnvalue_6 "0, 0, 0" "1.600000,1.600000,1.600000") "Undefined" "MultiplyWithRoot" 0 0)
          (Utilities|FlowControl|Delay 1.0)
          (Game|SpawnActorfromClass "/Game/LHW/Skill_Resouroes/Meteor/Meteor_stone.Meteor_stone_C" (Math|Transform|MakeTransform _returnvalue_7 "0, 0, 0" "3.000000,3.000000,2.000000") "Undefined" "MultiplyWithRoot" 0 0)
          (Utilities|FlowControl|Delay 5.0)
          (Actor|DestroyActor _returnvalue_10))
        (:then_1
          (Variables|/Script/UMG.Widget|SetRenderOpacity (Variables|/Game/LHW/ui/WBP_CharacterUi.WBP_CharacterUi_C|GetTextBlock_5 (Variables|/Game/LHW/BluePrint/LHW_playerGameMode.LHW_playerGameMode_C|GetCharacterUi (Variables|/Game/LHW/BluePrint/MyplayerCharacter.MyplayerCharacter_C|GetAs%20LHW%20Player%20Game%20Mode _asmyplayer_character_2))) 1.0)
          (bind (_direction _newtrack_0_2 _newtrack_1) (Timeline|Timeline_0 PlayFromStart)
            (:Update
              (Variables|/Game/LHW/ui/WBP_CharacterUi.WBP_CharacterUi_C|SetMeteorCoolDown (Variables|/Game/LHW/BluePrint/LHW_playerGameMode.LHW_playerGameMode_C|GetCharacterUi (Variables|/Game/LHW/BluePrint/MyplayerCharacter.MyplayerCharacter_C|GetAs%20LHW%20Player%20Game%20Mode _asmyplayer_character_2)) _newtrack_0_2)
              (Variables|/Game/LHW/ui/WBP_CharacterUi.WBP_CharacterUi_C|SetMeteorCoolDownText (Variables|/Game/LHW/BluePrint/LHW_playerGameMode.LHW_playerGameMode_C|GetCharacterUi (Variables|/Game/LHW/BluePrint/MyplayerCharacter.MyplayerCharacter_C|GetAs%20LHW%20Player%20Game%20Mode _asmyplayer_character_2)) (Math|Float|Truncate _newtrack_1)))
            (:Finished
              (Variables|/Script/UMG.Widget|SetRenderOpacity (Variables|/Game/LHW/ui/WBP_CharacterUi.WBP_CharacterUi_C|GetTextBlock_5 (Variables|/Game/LHW/BluePrint/LHW_playerGameMode.LHW_playerGameMode_C|GetCharacterUi (Variables|/Game/LHW/BluePrint/MyplayerCharacter.MyplayerCharacter_C|GetAs%20LHW%20Player%20Game%20Mode _asmyplayer_character_2))) 0.0))))))))

(event EventTick
  (params (DeltaSeconds :type Float%20%28single-precision%29)))

(fn ConstructionScript)

(fn SkillcancelHandler
  (params (second :type Float%20%28double-precision%29)))