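; Boss character that tracks health and combat phase as player attacks hit it.
; Overlaps with normal attack, meteor and ice colliders each set their own damage, then share one path that subtracts health and sets the phase from health thresholds, zero at death.
; BeginPlay creates the boss health bar widget, and Tick pushes current and max health to it.
; Attack montage and walk animation logic is present but never runs.
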(event EventBeginPlay
  (bind _returnvalue (UserInterface|CreateWidget "/Game/LHW/ui/WBP_BossHealthBar.WBP_BossHealthBar_C"))
  (UserInterface|Viewport|AddtoViewport _returnvalue 0)
  (Variables|Default|Sethpbar _returnvalue))

(event Collision|EventActorBeginOverlap
  (params (OtherActor :type Actor%20Object%20Reference))
  ;[0.15 0.15 0.15 0.5] 플레이어와 충돌시 HP 10감소
  (Utilities|FlowControl|Sequence
    (:then_0
      (Utilities|Casting|CastToBP_NormalAttack OtherActor)
      (Variables|Default|SetDamageHP 1000))
    (:then_1
      (Utilities|Casting|CastToBP_MeteorCollider OtherActor)
      (Variables|Default|SetDamageHP 5000))
    (:then_2
      (Utilities|Casting|CastToBP_IceCollider OtherActor)
      (Variables|Default|SetDamageHP 10000)))
  ;[0.15 0.15 0.15 0.5] HP에 따라 달라지는 Phase
  (Variables|Default|SetCurrentHP (- (Variables|Default|GetCurrentHP) (Variables|Default|GetDamageHP)))
  (if (>= (Variables|Default|GetCurrentHP) (* (Variables|Default|GetMaxHp) 0.7))
    (Variables|Default|SetPhase 1)
    (Development|PrintString "충돌! Phase 1")
    (elif (>= (Variables|Default|GetCurrentHP) (* (Variables|Default|GetMaxHp) 0.4))
      (Variables|Default|SetPhase 2)
      (Development|PrintString "충돌! Phase 2")
      (elif (> (Variables|Default|GetCurrentHP) 0.0)
        (Variables|Default|SetPhase 3)
        (Development|PrintString "충돌! Phase 3")
        (else
          (Variables|Default|SetPhase 0))))))

(event EventTick
  (params (DeltaSeconds :type Float%20%28single-precision%29))
  (bind _hpbar (Variables|Default|Gethpbar))
  (Variables|/Game/LHW/ui/WBP_BossHealthBar.WBP_BossHealthBar_C|SetBossCurrentHealth _hpbar (Variables|Default|GetCurrentHP))
  (Variables|/Game/LHW/ui/WBP_BossHealthBar.WBP_BossHealthBar_C|SetBossMaxHealth _hpbar (Variables|Default|GetMaxHp)))

(fn ConstructionScript)