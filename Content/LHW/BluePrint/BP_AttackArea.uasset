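; BP_AttackArea is an actor that acts as a flat attack-area marker beneath the player character.
; Each Tick casts the player to MyplayerCharacter and switches on its OnchageKey to pick one of two area sizes.
; In those two cases it moves to the player's position, lowered toward the feet, and scales in X and Y with a thin Z.
; Right mouse only prints a debug string.
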(event Collision|EventActorBeginOverlap
  (params (OtherActor :type Actor%20Object%20Reference)))

(event EventTick
  (params (DeltaSeconds :type Float%20%28single-precision%29))
  (bind _returnvalue (Game|GetPlayerCharacter 0))
  (bind _returnvalue_2 (Transformation|GetActorLocation _returnvalue))
  (bind (_x _y _z) (Math|Vector|BreakVector _returnvalue_2))
  (bind _asmyplayer_character (Utilities|Casting|CastToMyplayerCharacter (Game|GetPlayerCharacter 0)))
  (switch int (Variables|/Game/LHW/BluePrint/MyplayerCharacter.MyplayerCharacter_C|GetonchageKey _asmyplayer_character)
    (:1
      (Variables|Default|SetattackAreaSize "1.500000,1.500000,1.500000"))
    (:2
      (Variables|Default|SetattackAreaSize "2.000000,2.000000,2.000000")))
  (Transformation|SetActorLocation (Math|Vector|MakeVector _x _y (+ _z -9e+01)) false false)
  (Transformation|SetActorScale3D (Math|Vector|MakeVector (.x (Variables|Default|GetattackAreaSize)) (.y (Variables|Default|GetattackAreaSize)) 0.1)))

(event Input|MouseEvents|RightMouseButton
  (params (Key :type Key%20Structure :default "None"))
  (:Pressed
    (Development|PrintString "Hello")))

(fn ConstructionScript)