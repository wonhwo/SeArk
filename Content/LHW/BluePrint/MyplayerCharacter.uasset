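; Player mage character that aims at the cursor, fires normal attacks, casts icicle and meteor skills, dashes and zooms the camera.
; E or R spawns targeting circles that a left click turns into the spell, gated by mana and timer cooldowns.
; Damage causes knockback stun with a Space get-up, or death and game over.
; Timelines and handlers feed HP, MP and cooldown UI, while input toggling locks actions.
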(event EventBeginPlay
  ;[0.15 0.15 0.15 0.5] 게임모드 가져오기
  (bind _aslhw_player_game_mode (Utilities|Casting|CastToLHW_playerGameMode (Game|GetGameMode)))
  (Variables|Default|SetAs%20LHW%20Player%20Game%20Mode _aslhw_player_game_mode)
  ;[0.15 0.15 0.15 0.5] Dash UI 생성
  (bind _returnvalue (UserInterface|CreateWidget "/Game/LHW/ui/WBP_DashDelay.WBP_DashDelay_C"))
  (Variables|Default|SetDashDelayUI _returnvalue))

(event EventTick
  (params (DeltaSeconds :type Float%20%28single-precision%29))
  ;[0.15 0.15 0.15 0.5] 캐릭터 후딜 감지
  (Utilities|FlowControl|Sequence
    (:then_0
      (Variables|Default|SetSkillCanCel false)
      (Variables|Default|SetSendMesh (Variables|Character|GetMesh))
      (if (not (Variables|Default|GetisSkillCasting))
        (CallFunction|StartMovementPlayer)))
    (:then_1
      ;[0.15 0.15 0.15 0.5] 마나 재생
      (Utilities|FlowControl|Delay 1.0)
      (CallFunction|MPRegenerater 1e+01))))

(event Game|Damage|EventAnyDamage
  (params (Damage :type Float%20%28single-precision%29) (DamageType :type Damage%20Type%20Object%20Reference) (InstigatedBy :type Controller%20Object%20Reference) (DamageCauser :type Actor%20Object%20Reference))
  ;[0.15 0.15 0.15 0.5] 데미지 피격 이벤트 부분
  (CallFunction|HpuiHander Damage)
  (Variables|Default|SetDamage%20Causer DamageCauser)
  (if (> (Variables|Default|GetCurrentHP) 0.0)
    (CallFunction|HeavyHit)
    (Variables|Default|SetisStun true)
    ;[0.15 0.15 0.15 0.5] 스턴 상태 체크
    (Timeline|Timeline_0 PlayFromStart
      (:Update
        (if (Variables|Default|GetisGetUp)
          (Animation|PlayAnimMontage "/Game/LHW/LHW_Anim/MT_Getup.MT_Getup" 1.0 "None")
          (Variables|Default|SetisGetUp false)
          (Utilities|FlowControl|Delay 1.0)
          (CallFunction|StartMovementPlayer)
          (Variables|Default|SetisStun false)
          (Timeline|Timeline_0 Stop)))
      (:Finished
        ;[0.15 0.15 0.15 0.5] 기상기 부분
        (Animation|StopAnimMontage "/Game/LHW/LHW_Anim/BT_death.BT_death")
        (Animation|PlayAnimMontage "/Game/LHW/LHW_Anim/MT_Getup.MT_Getup" 1.0 "None")
        (Utilities|FlowControl|Delay 1.0)
        (CallFunction|StartMovementPlayer)
        (Variables|Default|SetisStun false)))
    (else
      (CallFunction|PlayerDeath))))

(event Input|ActionEvents|InputActionspace
  (params (Key :type Key%20Structure :default "None"))
  (bind _dashdelayui (Variables|Default|GetDashDelayUI))
  ;[0.15 0.15 0.15 0.5] Dash & GetUp
  ;;[0.15 0.15 0.15 0.5] 스페이스바 이벤트 구별하기
  (:Pressed
    (if (Variables|Default|GetisStun)
      (Variables|Default|SetisGetUp true)
      (elif (Variables|Default|GetDashDelay)
        (Variables|Default|SetSkillCanCel true)
        (Variables|Default|SetDashDelay false)
        (Utilities|FlowControl|Sequence
          (:then_0
            (CallFunction|ShowDashUiHandler))
          (:then_1
            ;;[0.15 0.15 0.15 0.5] dash ui progressbar
            (bind (_direction _newtrack_0 _text) (Timeline|Dash PlayFromStart)
              (:Update
                (Variables|/Game/LHW/ui/WBP_DashDelay.WBP_DashDelay_C|SetprograssValue _dashdelayui _newtrack_0)
                (Variables|/Game/LHW/ui/WBP_DashDelay.WBP_DashDelay_C|SettextValue _dashdelayui (Math|Float|Truncate _text)))
              (:Finished
                (Variables|Default|SetDashDelay true)
                (Widget|RemovefromParent _dashdelayui)))))))))

(event Input|ActionEvents|InputActionSkill
  (params (Key :type Key%20Structure :default "None"))
  (:Pressed
    ;[0.15 0.15 0.15 0.5] 키보드 입력 이후 어떤 키가 눌렸는지 판단후 크기에 맞게 마법진 생성
    (bind _output_get (Variables|Default|SetSkillKey Key))
    (if (Variables|Default|GetisClick)
      (Utilities|FlowControl|Sequence
        (:then_0
          (if (>= (Variables|Default|GetCurrentMp) 5e+01)
            (if (== _output_get "E")
              (if (Variables|Default|GetIceCoolDown)
                (Variables|Default|SetSkillKey "None" :!label _label)
                (else
                  (Variables|Default|SetonChageKey 1)
                  (Variables|Default|SetSkilRange "1.000000,1.000000,1.000000")
                  (bind (_newparam _newparam1) (CallFunction|SpawnMagicCircleHandler :!label _label_2)))))))
        (:then_1
          (if (>= (Variables|Default|GetCurrentMp) 1e+02)
            (if (== _output_get "R")
              (if (Variables|Default|GetMeteorCoolDown)
                (goto _label)
                (else
                  (Variables|Default|SetonChageKey 2)
                  (Variables|Default|SetSkilRange "6.500000,6.500000,6.500000")
                  (goto _label_2))))))))))

(event Input|ActionEvents|InputActionSkillCancel
  (params (Key :type Key%20Structure :default "None"))
  ;[0.15 0.15 0.15 0.5] 스킬 취소
  (:Pressed
    (Variables|Default|SetSkillCanCel true)
    (Variables|Default|SetSkillKey "None")
    (Utilities|IsValid (stale Input|ActionEvents|InputActionSkill _newparam)
      (:Is%20Valid
        (Utilities|FlowControl|Sequence
          (:then_0
            (Actor|DestroyActor (stale Input|ActionEvents|InputActionSkill _newparam))
            (Variables|Default|SetisClick true)
            (CallFunction|StartMovementPlayer))
          (:then_1
            (Actor|DestroyActor (stale Input|ActionEvents|InputActionSkill _newparam1))))))))

(event Input|MouseEvents|MouseWheelAxis
  (params (AxisValue :type Float%20%28single-precision%29))
  ;[0.15 0.15 0.15 0.5] 카메라 줌/인
  (CallFunction|CameraArmLenthHandler))

(event Input|MouseEvents|LeftMouseButton
  (params (Key :type Key%20Structure :default "None"))
  (bind _skillkey (Variables|Default|GetSkillKey))
  (bind _as_lhw_player_game_mode (Variables|Default|GetAs%20LHW%20Player%20Game%20Mode))
  (bind _characterui (Variables|/Game/LHW/BluePrint/LHW_playerGameMode.LHW_playerGameMode_C|GetCharacterUi _as_lhw_player_game_mode))
  (bind _textblock_6 (Variables|/Game/LHW/ui/WBP_CharacterUi.WBP_CharacterUi_C|GetTextBlock_6 _characterui))
  ;[0.15 0.15 0.15 0.5] 마우스 클릭이후 어떤 키가 눌렸는지 구별한 뒤 스킬 생성
  (:Pressed
    (if (Variables|Default|GetattackDelay)
      (CallFunction|CharacterfindMousePosition)
      (Utilities|FlowControl|Delay 0.05)
      (Utilities|IsValid (stale Input|ActionEvents|InputActionSkill _newparam)
        (:Is%20Valid
          (Utilities|FlowControl|Sequence
            (:then_0
              (if (== _skillkey "E")
                (CallFunction|Skill3)
                (CallFunction|Skill3)
                (CallFunction|Skill3)
                (CallFunction|MPHander 5e+01)
                ;[0.15 0.15 0.15 0.5] 얼음 ui 프로그래스바
                (Utilities|FlowControl|Sequence
                  (:then_0
                    ;[0.15 0.15 0.15 0.5] 마법진 파괴 부분
                    (Utilities|IsValid (stale Input|ActionEvents|InputActionSkill _newparam)
                      (:Is%20Valid
                        (Actor|DestroyActor (stale Input|ActionEvents|InputActionSkill _newparam))
                        (Actor|DestroyActor (stale Input|ActionEvents|InputActionSkill _newparam1))
                        (Variables|Default|SetisClick true :!label _label))))
                  (:then_1
                    (Class|TextBlock|SetOpacity _textblock_6 1.0)
                    (bind (_direction _newtrack_0 _newtrack_1) (Timeline|Timeline PlayFromStart)
                      (:Update
                        (Variables|/Game/LHW/ui/WBP_CharacterUi.WBP_CharacterUi_C|SetIceCoolDown _characterui _newtrack_0)
                        (Variables|/Game/LHW/ui/WBP_CharacterUi.WBP_CharacterUi_C|SetIceCoolText _characterui (Math|Float|Truncate _newtrack_1)))
                      (:Finished
                        (Class|TextBlock|SetOpacity _textblock_6 0.0)))))))
            (:then_1
              (if (== _skillkey "R")
                (CallFunction|SpawnMeteor)
                (Utilities|IsValid (stale Input|ActionEvents|InputActionSkill _newparam1)
                  (:Is%20Valid
                    (Actor|DestroyActor (stale Input|ActionEvents|InputActionSkill _newparam))
                    (Actor|DestroyActor (stale Input|ActionEvents|InputActionSkill _newparam1))
                    (goto _label)))))))
        (:Is%20Not%20Valid
          (if (and (Variables|Default|GetattackDelay) (Variables|Default|GetNormalAttackDelay))
            (CallFunction|StopMovementPlayer)
            (CallFunction|NormalAttact)
            (Utilities|FlowControl|Delay 0.2)
            (CallFunction|StartMovementPlayer)))))))

(fn ConstructionScript)

(fn Skill3
  (bind _attacareaob (Variables|Default|GetAttacAreaOb))
  (bind _returnvalue (Transformation|GetActorLocation _attacareaob))
  (bind _returnvalue_2 (Game|SpawnActorfromClass "/Game/LHW/Skill_Resouroes/ice/BP_Icicle.BP_Icicle_C" (Math|Transform|MakeTransform (+ (Transformation|GetActorLocation) (Math|Vector|MakeVector (Math|Conversions|ToFloat(Integer) (* (Class|KismetMathLibrary|RandomInteger64inRange -30 30) 10)) 0.0 2e+02)) "0, 0, 0" "0.300000,0.300000,0.300000") "Undefined" "OverrideRootScale" 0 0))
  (bind _output_get (Variables|Default|SetSpawnedIceActor _returnvalue_2))
  (Utilities|IsValid _output_get
    (:Is%20Valid
      (Variables|/Game/LHW/Skill_Resouroes/ice/BP_Icicle.BP_Icicle_C|SetTargetLocation _output_get _returnvalue)
      (Transformation|SetActorRotation _output_get (Math|Rotator|FindLookatRotation (Transformation|GetActorLocation _returnvalue_2) _returnvalue))
      (CallFunction|StopMovementPlayer)
      (Variables|Default|SetSkillKey "")
      (Variables|Default|SetIceCoolDown true)
      (Development|PrintString "쿨타임 3초 시작" true true "(R=1.000000,G=0.893634,B=0.349146,A=1.000000)")
      (Utilities|Time|SetTimerbyFunctionName 0 "CoolDownIce" 5.0))))

(fn SpawnMeteor
  (bind _attacareaob (Variables|Default|GetAttacAreaOb))
  (bind _returnvalue (Transformation|GetActorLocation _attacareaob))
  (Animation|PlayAnimMontage "/Game/LHW/Rig_Animation/MT_MeteorCasting.MT_MeteorCasting" 0.5 "None")
  (Game|SpawnActorfromClass "/Game/LHW/Skill_Resouroes/Meteor/BP_MeteorSkill.BP_MeteorSkill_C" (Math|Conversions|ToTransform(Vector) (Math|Vector|MakeVector (.x _returnvalue) (.y _returnvalue) (.z (Transformation|GetActorLocation (Game|GetPlayerCharacter 0))))) "Undefined" "MultiplyWithRoot" 0 0)
  (Variables|Default|SetSkillKey "")
  (Variables|Default|SetMeteorCoolDown true)
  (Utilities|Time|SetTimerbyFunctionName 0 "CoolDownTeteor" 1e+01))

(fn StopMovementPlayer
  (Variables|Default|SetisSkillCasting true)
  (Components|Movement|StopMovementImmediately (Variables|Character|GetCharacterMovement))
  (Input|DisableInput (Game|GetPlayerController 0) 0)
  (Variables|Default|SetNormalAttackDelay false))

(fn StartMovementPlayer
  (Input|EnableInput (Game|GetPlayerController 0) 0)
  (Variables|Default|SetNormalAttackDelay true))

(fn NormalAttact
  (bind _arrow1 (Variables|컴포넌트|GetArrow1))
  (bind _returnvalue (Transformation|GetWorldTransform _arrow1))
  (bind (_x _y _z) (Math|Vector|BreakVector (.location _returnvalue)))
  (CallFunction|CharacterfindMousePosition)
  (Animation|PlayAnimMontage "/Game/LHW/LHW_Anim/MT_Cast.MT_Cast" 2.0 "None")
  (bind _returnvalue_2 (Game|SpawnActorfromClass "/Game/LHW/Skill_Resouroes/NormalAttack/BP_NormalAttack.BP_NormalAttack_C" (Math|Transform|MakeTransform (Math|Vector|MakeVector _x _y _z) (.rotation _returnvalue) (.scale _returnvalue)) "Undefined" "MultiplyWithRoot" 0 0))
  (Transformation|SetActorRotation _returnvalue_2 (Math|Rotator|FindLookatRotation (Transformation|GetActorLocation) (Variables|Default|GetMousePosition))))

(fn GetMousePosition
  (Variables|Default|SetMousePosition (.ImpactPoint (Collision|BreakHitResult (.HitResult (Game|Player|GetHitResultUnderCursorbyChannel (Game|GetPlayerController 0) "TraceTypeQuery1" true))))))

(fn CharacterfindMousePosition
  (bind _returnvalue (Transformation|GetActorLocation))
  (bind _mouseposition (Variables|Default|GetMousePosition))
  (bind _returnvalue_2 (Math|Rotator|FindLookatRotation _returnvalue _mouseposition))
  (if (Variables|Default|GetNormalAttackDelay)
    (CallFunction|GetMousePosition)
    (Variables|Default|SetTargetRotation _returnvalue_2)
    (Transformation|SetActorRotation _returnvalue_2)))

(fn CoolDownIce
  (Development|PrintString "아이스에이지 쿨타운 끝" true true "(R=1.000000,G=0.956113,B=0.286401,A=1.000000)")
  (Variables|Default|SetIceCoolDown false))

(fn CoolDownTeteor
  (Development|PrintString "메테오 쿨타운 끝" true true "(R=1.000000,G=0.956113,B=0.286401,A=1.000000)")
  (Variables|Default|SetMeteorCoolDown false))

(fn DashHandler
  (Character|LaunchCharacter (+ (* (Transformation|GetActorForwardVector) "6000.000000,6000.000000,6000.000000") (Transformation|GetActorUpVector)) false false))

(fn HeavyHit
  (params (NewParam :type Enemy%20Sample%20Object%20Reference))
  (bind _damage_causer (Variables|Default|GetDamage%20Causer))
  (Utilities|IsValid _damage_causer
    (:Is%20Valid
      (CallFunction|StopMovementPlayer)
      (Animation|PlayAnimMontage "/Game/LHW/LHW_Anim/BT_death.BT_death" 2.0 "None")
      (Character|LaunchCharacter (* (Math|Vector|NegateVector (Math|Vector|Normalize (- (Transformation|GetActorLocation _damage_causer) (Transformation|GetActorLocation)))) (Variables|Default|GetKnockbackSpeed)) true false))))

(fn CameraArmLenthHandler
  (bind _springarmcomponent (Variables|Default|GetSpringArmComponent))
  (bind _targetarmlength (Variables|/Script/Engine.SpringArmComponent|GetTargetArmLength _springarmcomponent))
  (Class|PlayerCharacter|SetCameraArmLength (Math|Float|Clamp(Float) (Math|Interpolation|FInterpTo _targetarmlength (+ (* (Input|AxisValues|GetmouseWheel) (Variables|Default|GetzoomSpeed)) _targetarmlength) (Utilities|Time|GetWorldDeltaSeconds) 1.0) 1e+02 1e+03)))

(fn ShowDashUiHandler
  (bind _dashdelayui (Variables|Default|GetDashDelayUI))
  (CallFunction|StopMovementPlayer)
  (AddComponent|AddNiagaraComponent false)
  (Utilities|IsValid _dashdelayui
    (:Is%20Valid
      (UserInterface|Viewport|AddtoViewport _dashdelayui 0)
      (CallFunction|DashHandler)
      (CallFunction|StartMovementPlayer)
      (return))))

(fn SpawnMagicCircleHandler
  (bind _skilrange (Variables|Default|GetSkilRange))
  (bind _returnvalue (Math|Transform|MakeTransform (Math|Vector|MakeVector 0.0 0.0 0.0) "0, 0, 0" _skilrange))
  (Variables|Default|SetisClick false)
  (bind _returnvalue_2 (Game|SpawnActorfromClass "/Game/LHW/BluePrint/BP_AttackArea.BP_AttackArea_C" _returnvalue "Undefined" "MultiplyWithRoot" 0 0))
  (bind _returnvalue_3 (Game|SpawnActorfromClass "/Game/LHW/BluePrint/BP_Magic_Area.BP_Magic_Area_C" _returnvalue "Undefined" "MultiplyWithRoot" 0 0))
  (Utilities|IsValid _returnvalue_3
    (:Is%20Valid
      (Variables|Default|SetAttacAreaOb _returnvalue_3)
      (CallFunction|StopMovementPlayer)
      (return _returnvalue_3 _returnvalue_2))))

(fn HpuiHander
  (params (Damage :type Float%20%28double-precision%29))
  (bind _as_lhw_player_game_mode (Variables|Default|GetAs%20LHW%20Player%20Game%20Mode))
  (bind _characterui (Variables|/Game/LHW/BluePrint/LHW_playerGameMode.LHW_playerGameMode_C|GetCharacterUi _as_lhw_player_game_mode))
  (bind _output_get (Variables|Default|SetCurrentHP (- (Variables|Default|GetCurrentHP) Damage)))
  (Variables|/Game/LHW/ui/WBP_CharacterUi.WBP_CharacterUi_C|SetHP _characterui (Math|Float|Lerp 1.0 (Math|Float|Clamp(Float) (/ (Variables|Default|GetCurrentHP) (Variables|Default|GetMaxHP))) 1.0))
  (Variables|/Game/LHW/ui/WBP_CharacterUi.WBP_CharacterUi_C|SetHPText _characterui (Math|Float|Truncate _output_get)))

(fn MPHander
  (params (SubMp :type Float%20%28double-precision%29))
  (Variables|Default|SetCurrentMp (- (Variables|Default|GetCurrentMp) SubMp))
  (Variables|/Game/LHW/ui/WBP_CharacterUi.WBP_CharacterUi_C|SetMP (Variables|/Game/LHW/BluePrint/LHW_playerGameMode.LHW_playerGameMode_C|GetCharacterUi (Variables|Default|GetAs%20LHW%20Player%20Game%20Mode)) (Math|Float|Clamp(Float) (/ (Variables|Default|GetCurrentMp) (Variables|Default|GetMaxMP)))))

(fn MPRegenerater
  (params (addMp :type Float%20%28double-precision%29))
  (bind _as_lhw_player_game_mode (Variables|Default|GetAs%20LHW%20Player%20Game%20Mode))
  (bind _characterui (Variables|/Game/LHW/BluePrint/LHW_playerGameMode.LHW_playerGameMode_C|GetCharacterUi _as_lhw_player_game_mode))
  (if (< (Variables|Default|GetCurrentMp) (Variables|Default|GetMaxMP))
    (Variables|Default|SetCurrentMp (+ (Variables|Default|GetCurrentMp) addMp))
    (Variables|/Game/LHW/ui/WBP_CharacterUi.WBP_CharacterUi_C|SetMP _characterui (Math|Float|Clamp(Float) (/ (Variables|Default|GetCurrentMp) (Variables|Default|GetMaxMP))))
    (Variables|/Game/LHW/ui/WBP_CharacterUi.WBP_CharacterUi_C|SetMPText _characterui (Math|Float|Truncate (Variables|Default|GetCurrentMp)))))

(fn PlayerDeath
  (CallFunction|StopMovementPlayer)
  (Animation|PlayAnimMontage "/Game/LHW/LHW_Anim/MT_StandingDeath.MT_StandingDeath" 1.0 "None")
  (bind _returnvalue (UserInterface|CreateWidget "/Game/LHW/ui/WBP_GamemoOver.WBP_GamemoOver_C"))
  (UserInterface|Viewport|AddtoViewport _returnvalue 0))

(fn MapBreakHander
  (Game|SpawnActorfromClass "/Game/LHW/BluePrint/BP_ms.BP_ms_C" (Math|Transform|MakeTransform (Math|Vector|MakeVector 994.0 466.0 273.0) "0, 0, 0" "1.000000,1.000000,1.000000") "Undefined" "MultiplyWithRoot" 0 0)
  (Utilities|FlowControl|Sequence
    (:then_0
      (bind _returnvalue (Actor|GetActorOfClass "/Game/LHW/MerlinsCave/Blueprints/BP_Floor02.BP_Floor02_C"))
      (Utilities|IsValid _returnvalue
        (:Is%20Valid
          (Actor|DestroyActor _returnvalue))))
    (:then_1
      (bind _outactors (Actor|GetAllActorswithTag "wall"))
      (for _array_element _outactors
        (Utilities|IsValid _array_element
          (:Is%20Valid
            (Actor|DestroyActor _array_element)))))
    (:then_2
      (bind _outactors_2 (Actor|GetAllActorsOfClass "/Game/LHW/Map/BP_BossWall.BP_BossWall_C"))
      (for _array_element_2 _outactors_2
        (Collision|SetCollisionEnabled (Variables|/Game/LHW/Map/BP_BossWall.BP_BossWall_C|GetBox _array_element_2) "QueryAndPhysics")
        (Development|PrintString "Hello")))))